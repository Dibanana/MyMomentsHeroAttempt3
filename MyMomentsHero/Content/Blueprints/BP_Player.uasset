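; BP_Player is a flipbook-animated 2D player character that runs along its forward axis and jumps.
; It registers the PlayerInput Enhanced Input mapping on BeginPlay, then uses Movement and Jump actions to drive motion and swap idle, run and jump flipbooks.
; Sprite rotation flips facing by input sign.
; An IsJumping flag blocks run, idle and facing changes until landing restores the looping idle animation.
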(event `self.ReceiveBeginPlay`
  (bind _asplayer_controller (cast `PlayerController` (`self.GetController`)))
  (`EnhancedInputSubsystemInterface.AddMappingContext` (pcsubsystem `EnhancedInputLocalPlayerSubsystem` _asplayer_controller) "/Game/Blueprints/PlayerInput.PlayerInput" 0 (struct)))

(event `EnhancedInput|/Game/Blueprints/Movement`
  (params (ActionValue :type "Float (double-precision)") (ElapsedSeconds :type "Float (double-precision)") (TriggeredSeconds :type "Float (double-precision)") (InputAction :type "InputAction Object Reference" :default "/Game/Blueprints/Movement.Movement"))
  (bind _returnvalue (not (`self.IsJumping`)))
  (:`Triggered`
    (`self.AddMovementInput` (`self.GetActorForwardVector`) ActionValue)
    (if _returnvalue
      (`PaperFlipbookComponent.SetFlipbook` (`self.Sprite`) "/Game/Assets/Textures/Characters/Player/Flipbook/RunFlip.RunFlip")
      (if (> ActionValue 0.0)
        (`SceneComponent.K2_SetWorldRotation` :`self` (`self.Sprite`))
        (else
          (`SceneComponent.K2_SetWorldRotation` (`self.Sprite`) (struct :`Yaw` 180.0) false false)))))
  (:`Completed`
    (if _returnvalue
      (`PaperFlipbookComponent.SetFlipbook` (`self.Sprite`) "/Game/Assets/Textures/Characters/Player/Flipbook/IdleFlip.IdleFlip"))))

(event `EnhancedInput|/Game/Blueprints/Jump`
  (params (ActionValue :type Boolean) (ElapsedSeconds :type "Float (double-precision)") (TriggeredSeconds :type "Float (double-precision)") (InputAction :type "InputAction Object Reference" :default "/Game/Blueprints/Jump.Jump"))
  (bind _sprite (`self.Sprite`))
  (:`Triggered`
    (set `self.IsJumping` true)
    (`self.Jump`)
    (`PaperFlipbookComponent.SetLooping` _sprite false)
    (`PaperFlipbookComponent.SetFlipbook` _sprite "/Game/Assets/Textures/Characters/Player/Flipbook/Jumpflip.Jumpflip")))

(event `self.OnLanded`
  (params (Hit :type "HitResult Structure (by ref)"))
  (bind _sprite (`self.Sprite`))
  (set `self.IsJumping` false)
  (`PaperFlipbookComponent.SetLooping` _sprite true)
  (`PaperFlipbookComponent.Play` _sprite)
  (`PaperFlipbookComponent.SetFlipbook` _sprite "/Game/Assets/Textures/Characters/Player/Flipbook/IdleFlip.IdleFlip"))

(fn `UserConstructionScript`)